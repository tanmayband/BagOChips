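; InteractableBP_Door is an interactable door that swings open or closed when the player interacts with it.
; Interact runs the parent behavior, then calls ToggleDoor, which plays or reverses the ToggleDoorAnim timeline based on the Open flag.
; The timeline's alpha lerps the Door component's relative rotation through a quarter turn, and the flag flips when the animation finishes.
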(event Custom|ToggleDoor
  (if (Variables|Default|GetOpen?)
    (bind _alpha (Timeline|ToggleDoorAnim Reverse)
      (:Update
        (Transformation|SetRelativeRotation (Variables|Default|GetDoor) (Math|Rotator|Lerp(Rotator) "0, 0, 0" "0,-90.000000, 0" _alpha) false false))
      (:Finished
        (Variables|Default|SetOpen? (not (Variables|Default|GetOpen?)))))
    (else
      (Timeline|ToggleDoorAnim Play))))

(event EventBeginPlay
  (|CallParentFunction) ; This node is disabled and will not be called.\nDrag off pins to build functionality.
)

(event Collision|EventActorBeginOverlap
  (params (OtherActor :type Actor%20Object%20Reference))
  (|CallParentFunction OtherActor) ; This node is disabled and will not be called.\nDrag off pins to build functionality.
)

(event EventTick
  (params (DeltaSeconds :type Float%20%28single-precision%29))
  (|CallParentFunction DeltaSeconds) ; This node is disabled and will not be called.\nDrag off pins to build functionality.
)

(fn ConstructionScript
  (|CallParentFunction))

(fn Interact
  (|CallParentFunction)
  (CallFunction|ToggleDoor))