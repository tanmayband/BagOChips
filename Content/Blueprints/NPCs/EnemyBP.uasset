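; EnemyBP is an enemy NPC that drains the player's food on contact and is damaged by the player's chip vision.
; While chip vision is on, Tick deals damage over time if the player camera is within its current radius, using a squared-distance check.
; Overlapping the box with the player's camera or hand empties their food level.
; Damage flattens the enemy's Z scale as health drops; death only prints a debug message.
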(event OnComponentBeginOverlap(Box)
  (params (OverlappedComponent :type Primitive%20Component%20Object%20Reference) (OtherActor :type Actor%20Object%20Reference) (OtherComp :type Primitive%20Component%20Object%20Reference) (OtherBodyIndex :type Integer) (bFromSweep :type Boolean) (SweepResult :type Hit%20Result%20Structure%20%28by%20ref%29))
  (bind _asplayer_hand_bp (Utilities|Casting|CastToPlayerHandBP OtherActor))
  (if (and (CallFunction|IsAlive?) (or (== OtherComp (Variables|/Game/Blueprints/Player/PlayerHandBP.PlayerHandBP_C|GetCamera _asplayer_hand_bp)) (== OtherComp (Variables|/Game/Blueprints/Player/PlayerHandBP.PlayerHandBP_C|GetHand _asplayer_hand_bp))))
    (Default|UpdateHunger _asplayer_hand_bp (* (Variables|/Game/Blueprints/Player/PlayerHandBP.PlayerHandBP_C|GetCurrentFoodLevel _asplayer_hand_bp) -1.0))))

(event Custom|ChipVisionToggledEvent
  (params (Enabled? :type Boolean))
  (Variables|Default|SetChipVisionOn? Enabled?))

(event EventBeginPlay
  (EventDispatchers|AssignChipVisionToggledEvent (CallFunction|GetMyGameMode) (delegate Custom|ChipVisionToggledEvent))
  (Variables|Default|SetInitialScale (Variables|/Script/Engine.SceneComponent|GetRelativeScale3D (Variables|Default|GetDefaultSceneRoot))))

(event Collision|EventActorBeginOverlap
  (params (OtherActor :type Actor%20Object%20Reference)))

(event EventTick
  (params (DeltaSeconds :type Float%20%28single-precision%29))
  (if (and (Variables|Default|GetChipVisionOn?) (CallFunction|IsAlive?))
    (bind _asplayer_hand_bp (Utilities|Casting|CastToPlayerHandBP (Game|Player|GetPlayerPawn 0)))
    (if (CallFunction|CompareDistancetoPlayerComponent (Variables|/Game/Blueprints/Player/PlayerHandBP.PlayerHandBP_C|GetCamera _asplayer_hand_bp) (Variables|/Game/Blueprints/Player/PlayerHandBP.PlayerHandBP_C|GetChipVisionCurrentRadius _asplayer_hand_bp))
      (CallFunction|TakeDamage (* DeltaSeconds 1.0)))))

(fn ConstructionScript)

(fn TakeDamage
  (params (DamageAmount :type Float%20%28single-precision%29))
  (bind _initialscale (Variables|Default|GetInitialScale))
  (if (> (- (Variables|Default|GetHealth) DamageAmount) 0.0)
    (Variables|Default|SetHealth (- (Variables|Default|GetHealth) DamageAmount))
    (Transformation|SetRelativeScale3D (Variables|Default|GetDefaultSceneRoot) (Math|Vector|MakeVector (.x _initialscale) (.y _initialscale) (Math|Float|Lerp 0.3 (.z _initialscale) (/ (Variables|Default|GetHealth) 1e+01))))
    (else
      (Variables|Default|SetHealth 0.0)
      (CallFunction|EnemyDie))))

(fn EnemyDie
  (Development|PrintString "DED " true true "(R=1.000000,G=0.014181,B=0.000000,A=1.000000)"))

(fn IsAlive?
  (return (> (Variables|Default|GetHealth) 0.0)))

(fn CompareDistancetoPlayerComponent
  (params (PlayerComponent :type Scene%20Component%20Object%20Reference) (Distance :type Float%20%28single-precision%29))
  (return (<= (Class|KismetMathLibrary|VectorDistanceSquared (Transformation|GetActorLocation) (Transformation|GetWorldLocation PlayerComponent)) (Math|Float|Square Distance))))