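; Monster NPC made of a random cluster of floating mesh pieces that tumbles as it homes in on the player.
; The construction script rebuilds the collisionless pieces with random meshes and transforms, tagging them for custom depth stencil.
; While ToAnimate is set, Tick interpolates between random rotations and moves toward the player by a frame-rate-dependent step.
; Taking damage activates a VFX and slows both motions through SpeedScale until StopTakingDamage restores them.
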(event EventBeginPlay
  (|CallParentFunction))

(event Collision|EventActorBeginOverlap
  (params (OtherActor :type Actor%20Object%20Reference))
  (|CallParentFunction OtherActor) ; This node is disabled and will not be called.\nDrag off pins to build functionality.
)

(event EventTick
  (params (DeltaSeconds :type Float%20%28single-precision%29))
  (|CallParentFunction DeltaSeconds)
  (if (Variables|Animation|GetToAnimate?)
    (Utilities|FlowControl|Sequence
      (:then_0
        (if (not (Variables|Animation|GetRotationOngoing?))
          (Variables|Animation|SetLastRotation (Transformation|GetActorRotation))
          (Variables|Animation|SetNewRotation (Math|Random|RandomRotator true))
          (Variables|Animation|SetRotationOngoing? true)
          (Variables|Animation|SetRotationProgress 0.0)
          (else
            (bind _output_get (Variables|Animation|SetRotationProgress (Math|Float|Clamp(Float) (+ (Variables|Animation|GetRotationProgress) (* DeltaSeconds (* (Variables|Animation|GetRotationSpeed) (Variables|Animation|GetSpeedScale)))))))
            (Transformation|SetActorRotation (Math|Rotator|Lerp(Rotator) (Variables|Animation|GetLastRotation) (Variables|Animation|GetNewRotation) _output_get))
            (Variables|Animation|SetRotationOngoing? (< (Variables|Animation|GetRotationProgress) 1.0)))))
      (:then_1
        (Transformation|SetActorLocation (CallFunction|GetPointatDistanceAlongLine (Transformation|GetActorLocation) (CallFunction|GetPlayerLocation) (* (Variables|Animation|GetMovementSpeed) (Variables|Animation|GetSpeedScale))) false false)))))

(fn ConstructionScript
  (bind _monsterpiecescomponents (Variables|Default|GetMonsterPiecesComponents))
  (bind _monsterpiecesmeshes (Variables|Default|GetMonsterPiecesMeshes))
  (|CallParentFunction)
  (for _array_element _monsterpiecescomponents
    (Components|DestroyComponent _array_element))
  (Utilities|Array|Clear _monsterpiecescomponents)
  (for _index (range 0 (- (Variables|Default|GetNumPieces) 1))
    (bind _returnvalue (AddComponent|AddStaticMeshComponent false (Math|Transform|MakeTransform (Math|Vector|MakeVector (Math|Random|RandomFloatinRange -2e+02 2e+02) (Math|Random|RandomFloatinRange -2e+02 2e+02) (Math|Random|RandomFloatinRange -1e+02 1e+02)) (Math|Random|RandomRotator false) "1.000000,1,1")))
    (Utilities|Array|Add (Variables|Default|GetMonsterPiecesComponents) _returnvalue)
    (Components|StaticMesh|SetStaticMesh _returnvalue (Utilities|Array|Get(acopy) _monsterpiecesmeshes (Math|Random|RandomInteger (Utilities|Array|Length _monsterpiecesmeshes))))
    (Rendering|Material|SetMaterial _returnvalue 0 "/Engine/BasicShapes/BasicShapeMaterial.BasicShapeMaterial")
    (Rendering|SetRenderCustomDepth _returnvalue true)
    (Rendering|SetCustomDepthStencilValue _returnvalue 3)
    (Collision|SetCollisionEnabled _returnvalue "NoCollision")))

(fn TakeDamage
  (params (DamageAmount :type Float%20%28single-precision%29))
  (Components|Activation|Activate (Variables|Default|GetDamageVFX) false)
  (Variables|Animation|SetSpeedScale 0.3))

(fn StopTakingDamage
  (Components|Activation|Deactivate (Variables|Default|GetDamageVFX))
  (Variables|Animation|SetSpeedScale 1.0))