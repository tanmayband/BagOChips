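; ActorUtils is a utility Blueprint with a single function that tests whether an actor appears near the centre of the screen.
; It projects the actor's bounds origin, child actors included, to screen space through player controller 0.
; It returns true when both screen coordinates are positive and the point lies within a fixed pixel radius of the viewport centre, compared by squared distance.
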(fn CheckActorNearScreenCentre
  (params (Actor :type Actor%20Object%20Reference))
  (bind _origin (Collision|GetActorBounds Actor false true))
  (bind _returnvalue (Game|GetPlayerController 0))
  (bind _screenlocation (Class|PlayerController|ProjectWorldLocationtoScreen _returnvalue _origin false))
  (bind (_x _y) (Math|Vector2D|BreakVector2D _screenlocation))
  (return (Math|Boolean|ANDBoolean (> _x 0.0) (> _y 0.0) (<= (Class|KismetMathLibrary|DistanceSquared2D _screenlocation (/ (Viewport|GetViewportSize) 2.0)) (Math|Float|Square 1.5e+02)))))