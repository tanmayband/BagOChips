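; MathUtils is a set of math helper functions for enum bitmasks and points on lines.
; ConvertEnumToBitmaskInt turns an enum byte into a single-bit flag by raising two to its index, standing in for a left shift.
; CompareBitmaskToEnum uses that flag to test whether a bitmask contains the enum value.
; GetPointAtDistanceAlongLine offsets a start point by a distance along the unit direction toward an end point.
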(fn ConvertEnumtoBitmaskInt
  (params (EnumByte :type Byte))
  (return (* 1 (Math|Float|Truncate (Math|Float|Power 2.0 (Math|Conversions|ToFloat(Integer) (Math|Conversions|ToInteger(Byte) EnumByte)))))))

(fn CompareBitmasktoEnum
  (params (Bitmask :type Integer) (EnumByte :type Byte))
  (return (> (Class|KismetMathLibrary|AndIntInt Bitmask (CallFunction|ConvertEnumtoBitmaskInt EnumByte)) 0)))

(fn GetPointatDistanceAlongLine
  (params (StartPoint :type Vector) (EndPoint :type Vector) (Distance :type Float%20%28single-precision%29))
  (return (+ StartPoint (* (Math|Vector|GetUnitDirection(Vector) StartPoint EndPoint) Distance))))